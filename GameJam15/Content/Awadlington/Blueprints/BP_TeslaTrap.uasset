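; BP_TeslaTrap is a tesla trap that periodically stuns the player while they stay inside its trigger sphere.
; Overlap by the cached player pawn starts a shock that disables input, plays a zap and makes the sphere emissive for a brief delay.
; Each shock then restores both and sets a looping timer for the next.
; End overlap clears that timer, though leaving mid-shock does not prevent it being set afterwards.
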(event OnComponentBeginOverlap(TriggerSphere)
  (params (OverlappedComponent :type Primitive%20Component%20Object%20Reference) (OtherActor :type Actor%20Object%20Reference) (OtherComp :type Primitive%20Component%20Object%20Reference) (OtherBodyIndex :type Integer) (bFromSweep :type Boolean) (SweepResult :type Hit%20Result%20Structure%20%28by%20ref%29))
  (if (== OtherActor (Variables|Default|GetPlayerRef))
    (CallFunction|ShockPlayer)))

(event OnComponentEndOverlap(TriggerSphere)
  (params (OverlappedComponent :type Primitive%20Component%20Object%20Reference) (OtherActor :type Actor%20Object%20Reference) (OtherComp :type Primitive%20Component%20Object%20Reference) (OtherBodyIndex :type Integer))
  (if (== OtherActor (Variables|Default|GetPlayerRef))
    (Utilities|Time|ClearandInvalidateTimerbyHandle (Variables|Default|GetTimerHandle))))

(event Custom|ShockPlayer
  (bind _playerref (Variables|Default|GetPlayerRef))
  (Rendering|Material|SetMaterial (Variables|Default|GetSphere) 0 "/Engine/ArtTools/RenderToTexture/Materials/Debug/M_Emissive_Constant.M_Emissive_Constant")
  (Input|DisableInput _playerref (Game|GetPlayerController 0))
  (Audio|PlaySound2D "/Game/Awadlington/SFX/Tesla_Zap.Tesla_Zap" 1.0 1.0 0.0 0 0)
  (Utilities|FlowControl|Delay 1.0)
  (Rendering|Material|SetMaterial (Variables|Default|GetSphere) 0 "/Game/StarterContent/Materials/M_Glass.M_Glass")
  (Input|EnableInput _playerref (Game|GetPlayerController 0))
  (bind _returnvalue (Utilities|Time|SetTimerbyEvent (delegate Custom|ShockTimer) 5.0 true))
  (Variables|Default|SetTimerHandle _returnvalue))

(event Custom|ShockTimer
  (CallFunction|ShockPlayer))

(event EventBeginPlay
  (bind _asbp_third_person_character (Utilities|Casting|CastToBP_ThirdPersonCharacter (Game|Player|GetPlayerPawn 0)))
  (Variables|Default|SetPlayerRef _asbp_third_person_character))

(fn ConstructionScript)